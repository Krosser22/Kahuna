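; BP_HumanCharacter is the main human character Blueprint, handling pause menu display and audio listener placement.
; ActivePauseMenu creates and caches the pause widget on first use, switches to UI-only input with a cursor, hides the HUD widget and pauses the game.
; BeginPlay attaches the player controller's audio listener to the character mesh.
; A disconnected Life check that would open the MechanicTest level never runs.
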(event `self.ReceiveTick`
  (params (DeltaSeconds :type "Float (single-precision)")))

(event `self.ActivePauseMenu`
  (bind _returnvalue (`GameplayStatics.GetPlayerController` 0))
  (bind _pausemenureference (`self.PauseMenuReference`))
  ;[1 1 1] Display Pause Menu
  ;;[1 1 1] If it is the first time we access to the pause menu, it will create it and store it.
  (`/Engine/EditorBlueprintResources/StandardMacros.IsValid` (`self.PauseMenuReference`)
    (:`Is Valid`
      _)
    (:`Is Not Valid`
      (bind _returnvalue_2 (`|CreateWidget` "/Game/Game/UI/BP_PauseMenu.BP_PauseMenu_C"))
      (set `self.PauseMenuReference` _returnvalue_2)))
  (`WidgetBlueprintLibrary.SetInputMode_UIOnlyEx` (`GameplayStatics.GetPlayerController` 0) _pausemenureference)
  (`UserWidget.AddToViewport` _pausemenureference 0)
  (bind _asbp_hud (cast `/Game/Game/UI/BP_HUD` (`PlayerController.GetHUD` _returnvalue)))
  (`Widget.SetVisibility` (`/Game/Game/UI/BP_HUD.HUDUIReference` _asbp_hud) "Hidden")
  (set `PlayerController.bShowMouseCursor` true _returnvalue)
  (`GameplayStatics.SetGamePaused` true))

(event `self.ReceiveBeginPlay`
  ;[1 1 1] Set Audio
  (`PlayerController.SetAudioListenerOverride` :`self` (`GameplayStatics.GetPlayerController` 0) :`AttachToComponent` (`self.Mesh`)))

(fn `UserConstructionScript`)