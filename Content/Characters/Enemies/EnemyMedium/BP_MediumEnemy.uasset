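; Medium enemy character that spots the human player, chases them and deals melee damage.
; Pawn sensing or sight-box overlap sets PlayerSpotted, and leaving the box clears it.
; While spotted, Tick yaws the capsule toward the player and walks forward at reduced input.
; Hurt-box overlaps track attack range, and meleeAttack, not called within this graph, damages the first human character inside.
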(event `self.PawnSensing.OnSeePawn`
  (params (Pawn :type "Pawn Object Reference"))
  ;[1 1 1] Enemy_Vision_States
  (cast `/Game/Characters/Main/BP_HumanCharacter` Pawn)
  (set `self.Player_Spotted` true))

(event `melee Attack`
  ;[1 1 1] Enemy_Vision_States
  (for _array_element (`PrimitiveComponent.GetOverlappingActors` (`self.EnemyEasy_HurtBox`) null)
    (bind _asbp_human_character (cast `/Game/Characters/Main/BP_HumanCharacter` _array_element))
    (`GameplayStatics.ApplyDamage` _asbp_human_character 100.0)
    (break)))

(event `self.EnemyEasy_SightBox.OnComponentBeginOverlap`
  (params (OverlappedComponent :type "PrimitiveComponent Object Reference") (OtherActor :type "Actor Object Reference") (OtherComp :type "PrimitiveComponent Object Reference") (OtherBodyIndex :type Integer) (bFromSweep :type Boolean) (SweepResult :type "HitResult Structure (by ref)"))
  ;[1 1 1] Enemy_Vision_States
  (cast `/Game/Characters/Main/BP_HumanCharacter` OtherActor)
  (set `self.Player_Spotted` true))

(event `self.EnemyEasy_SightBox.OnComponentEndOverlap`
  (params (OverlappedComponent :type "PrimitiveComponent Object Reference") (OtherActor :type "Actor Object Reference") (OtherComp :type "PrimitiveComponent Object Reference") (OtherBodyIndex :type Integer))
  ;[1 1 1] Enemy_Vision_States
  (cast `/Game/Characters/Main/BP_HumanCharacter` OtherActor)
  (set `self.Player_Spotted` false))

(event `self.EnemyEasy_HurtBox.OnComponentBeginOverlap`
  (params (OverlappedComponent :type "PrimitiveComponent Object Reference") (OtherActor :type "Actor Object Reference") (OtherComp :type "PrimitiveComponent Object Reference") (OtherBodyIndex :type Integer) (bFromSweep :type Boolean) (SweepResult :type "HitResult Structure (by ref)"))
  ;[1 1 1] Enemy_Vision_States
  (cast `/Game/Characters/Main/BP_HumanCharacter` OtherActor)
  (set `self.Player_In_Attack_Range` true))

(event `self.EnemyEasy_HurtBox.OnComponentEndOverlap`
  (params (OverlappedComponent :type "PrimitiveComponent Object Reference") (OtherActor :type "Actor Object Reference") (OtherComp :type "PrimitiveComponent Object Reference") (OtherBodyIndex :type Integer))
  ;[1 1 1] Enemy_Vision_States
  (cast `/Game/Characters/Main/BP_HumanCharacter` OtherActor)
  (set `self.Player_In_Attack_Range` false))

(event `self.ReceiveTick`
  (params (DeltaSeconds :type "Float (single-precision)"))
  ;[1 1 1] Enemy_Moving+Rotation
  (if (`self.Player_Spotted`)
    (`SceneComponent.K2_SetWorldRotation` (`self.CapsuleComponent`) (`KismetMathLibrary.MakeRotator` 0.0 0.0 (.yaw (`KismetMathLibrary.FindLookAtRotation` (`self.K2_GetActorLocation`) (`self.K2_GetActorLocation` (`GameplayStatics.GetPlayerCharacter` 0))))) false false)
    (`self.AddMovementInput` (`SceneComponent.GetForwardVector` (`self.CapsuleComponent`)) 0.3)))

(fn `UserConstructionScript`)